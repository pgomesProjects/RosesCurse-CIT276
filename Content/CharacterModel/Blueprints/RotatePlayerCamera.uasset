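; RotatePlayerCamera is a trigger volume that turns the side-scroller character at a corner by passing it a new angle.
; BeginPlay picks start and end barriers from four directional options and opens the start one.
; On capsule overlap it sets the turn flag, ignores move input, swaps the blocking barrier and centers the player.
; Actor end overlap alternates the angle by 90 degrees for the next pass.
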(event `self.ReceiveBeginPlay`
  ;[1 0 0.009094] Set The Barriers For Rotation: (Key: 0 = Front, 1 = Right, 2 = Back, 3 = Left)
  (switch `int` (`self.StartBarrierUp`)
    (:`Default`
      (bind _output_get (set `self.StartBarrier` (`self.ForwardBarrier`) :!label _label))
      (`PrimitiveComponent.SetCollisionEnabled` _output_get "NoCollision"))
    (:`0`
      (goto _label))
    (:`1`
      (bind _output_get_2 (set `self.StartBarrier` (`self.RightBarrier`)))
      (`PrimitiveComponent.SetCollisionEnabled` _output_get_2 "NoCollision"))
    (:`2`
      (bind _output_get_3 (set `self.StartBarrier` (`self.BackwardBarrier`)))
      (`PrimitiveComponent.SetCollisionEnabled` _output_get_3 "NoCollision"))
    (:`3`
      (bind _output_get_4 (set `self.StartBarrier` (`self.LeftBarrier`)))
      (`PrimitiveComponent.SetCollisionEnabled` _output_get_4 "NoCollision")))
  (switch `int` (`self.EndBarrierUp`)
    (:`Default`
      (set `self.EndBarrier` (`self.ForwardBarrier`) :!label _label_2))
    (:`0`
      (goto _label_2))
    (:`1`
      (set `self.EndBarrier` (`self.RightBarrier`)))
    (:`2`
      (set `self.EndBarrier` (`self.BackwardBarrier`)))
    (:`3`
      (set `self.EndBarrier` (`self.LeftBarrier`))))
  (set `self.CurrentBarrier` (`self.EndBarrier`)))

(event `self.Volume.OnComponentBeginOverlap`
  (params (OverlappedComponent :type "PrimitiveComponent Object Reference") (OtherActor :type "Actor Object Reference") (OtherComp :type "PrimitiveComponent Object Reference") (OtherBodyIndex :type Integer) (bFromSweep :type Boolean) (SweepResult :type "HitResult Structure (by ref)"))
  ;[1 1 1] When The Player Overlaps, Allow Them To Turn And Temporarily Ignore Movement
  (bind _asside_scroller_character (cast `/Game/CharacterModel/SideScrollerCharacter` OtherActor))
  (if (== (`Character.CapsuleComponent` _asside_scroller_character) OtherComp)
    (set `/Game/CharacterModel/SideScrollerCharacter.Turn` true _asside_scroller_character)
    (set `/Game/CharacterModel/SideScrollerCharacter.PlayerAngle` (`self.Angle`) _asside_scroller_character)
    (`KismetSystemLibrary.PrintString` "Begin Overlap")
    (`Controller.SetIgnoreMoveInput` (`GameplayStatics.GetPlayerController` 0) true)
    (`PrimitiveComponent.SetCollisionEnabled` (`self.CurrentBarrier`) "NoCollision")
    (if (== (`self.CurrentBarrier`) (`self.StartBarrier`))
      (set `self.CurrentBarrier` (`self.EndBarrier`))
      (else
        (set `self.CurrentBarrier` (`self.StartBarrier`))))
    (`PrimitiveComponent.SetCollisionEnabled` (`self.CurrentBarrier`) "QueryAndPhysics")
    (`SceneComponent.K2_SetWorldLocation` OtherComp (`KismetMathLibrary.MakeVector` (.x (`SceneComponent.K2_GetComponentLocation` (`self.Spawn`))) (.y (`SceneComponent.K2_GetComponentLocation` (`self.Spawn`))) (.z (`self.K2_GetActorLocation` _asside_scroller_character))) true true)))

(event `self.ReceiveActorEndOverlap`
  (params (OtherActor :type "Actor Object Reference"))
  ;[1 1 1] When The Player Leaves The Overlap, If They Turn Left, Add 90 Degrees To The Angle. If Not, Subtract 90 Degrees
  (cast `/Game/CharacterModel/SideScrollerCharacter` OtherActor)
  (if (`self.IsTurnLeft?`)
    (set `self.Angle` (+ (`self.Angle`) 90.0))
    (set `self.IsTurnLeft?` false)
    (else
      (set `self.Angle` (- (`self.Angle`) 90.0))
      (set `self.IsTurnLeft?` true)))
  (`KismetSystemLibrary.PrintString` "End Overlap"))

(fn `UserConstructionScript`)