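; CheckForEnemies is an actor that ends the demo once its AllEnemies array is empty.
; It checks the array length every Tick, and nothing in its graphs fills or prunes the array.
; When empty, it shows the DemoEnd widget, sets IsGameEnd on PlayerGameMode, disables player input and destroys itself.
; A failed game mode cast stops the sequence after the widget appears.
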(event `self.ReceiveTick`
  (params (DeltaSeconds :type "Float (single-precision)"))
  (bind _returnvalue (`GameplayStatics.GetPlayerController` 0))
  (if (== (`KismetArrayLibrary.Array_Length` (`self.AllEnemies`)) 0)
    (bind _returnvalue_2 (`|CreateWidget` "/Game/Maps/TutorialLevel/Blueprints/DemoEnd.DemoEnd_C" _returnvalue))
    (`UserWidget.AddToViewport` _returnvalue_2 0)
    (bind _asplayer_game_mode (cast `/Game/CharacterModel/PlayerGameMode` (`GameplayStatics.GetGameMode`)))
    (set `/Game/CharacterModel/PlayerGameMode.isGameEnd` true _asplayer_game_mode)
    (`self.DisableInput` (`GameplayStatics.GetPlayerCharacter` 0) _returnvalue)
    (`self.K2_DestroyActor`)))

(fn `UserConstructionScript`)