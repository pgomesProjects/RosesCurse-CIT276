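; One-shot trigger actor that shows a tutorial popup when the player overlaps it.
; On overlap with a PlayerModel_Blueprint, it removes any tutorial widget the player already references, so the new popup replaces it.
; It then passes its category and info text to OpenTutorialPopup on the PlayerGameMode and destroys itself.
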(event `self.ReceiveActorBeginOverlap`
  (params (OtherActor :type "Actor Object Reference"))
  ;[1 1 1] Show The New Tutorial Popup and Replace Any Existing Ones
  (bind _asplayer_model_blueprint (cast `/Game/CharacterModel/PlayerModel_Blueprint` OtherActor))
  (bind _tutorial_widget (`/Game/CharacterModel/PlayerModel_Blueprint.Tutorial Widget` _asplayer_model_blueprint))
  (if (not (== _tutorial_widget null))
    (`Widget.RemoveFromParent` _tutorial_widget))
  (`/Game/CharacterModel/PlayerGameMode.OpenTutorialPopup` (cast `/Game/CharacterModel/PlayerGameMode` (`GameplayStatics.GetGameMode`) :!pure true) (`self.TutorialCategoryText`) (`self.TutorialText`))
  (`self.K2_DestroyActor`))

(fn `UserConstructionScript`)