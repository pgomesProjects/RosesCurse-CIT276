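; Tutorial level Blueprint that shows a starting tutorial popup when play begins.
; If ShowTutorial is set, BeginPlay passes its category and body text to OpenTutorialPopup on PlayerGameMode.
; It then sets a new objective through the same game mode if ShowObjective is also set, so no objective appears when the tutorial is off.
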(event `self.ReceiveBeginPlay`
  (bind _asplayer_game_mode (cast `/Game/CharacterModel/PlayerGameMode` (`GameplayStatics.GetGameMode`) :!pure true))
  (if (`self.ShowTutorial?`)
    (`/Game/CharacterModel/PlayerGameMode.OpenTutorialPopup` _asplayer_game_mode (`self.TutorialCategoryText`) (`self.TutorialText`))
    (if (`self.ShowObjective?`)
      (`/Game/CharacterModel/PlayerGameMode.NewObjective` _asplayer_game_mode (`self.ObjectiveText`)))))

(event `self.ReceiveTick`
  (params (DeltaSeconds :type "Float (single-precision)")))

(fn `UserConstructionScript`)